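; Mouse-driven tool pawn for the fluid simulation, tracing under the cursor to place a brush preview and spawn FakeDecal actors on left click.
; Right hold feeds the hit position to BP_FluidSimulation_01; wheel and A/Z adjust brush size and opacity.
; Tick's flow-map painting and obstacle-velocity branch is inactive because Pressed is never set true.
; Number keys debug-select the child-actor radial menu, whose events only print.
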(event `self.ReceiveBeginPlay`
  ;[1 1 1] On Begin Play
  (set `PlayerController.bShowMouseCursor` true (`GameplayStatics.GetPlayerController` 0))
  (bind _outactors (`GameplayStatics.GetAllActorsOfClass` "/Volumetrics/Tools/FluidSimulation/Blueprints/BP_FluidSimulation_01.BP_FluidSimulation_01_C"))
  (set `self.FluidSimBP` (`|GetArrayItem` _outactors))
  (bind _outactors_2 (`GameplayStatics.GetAllActorsOfClass` "/ShaderBits-GDC-Pack/FlowMapPainter/BP_PaintFlowMap.BP_PaintFlowMap_C"))
  (set `self.FlowMapBP` (`|GetArrayItem` _outactors_2))
  (bind _returnvalue (`PrimitiveComponent.CreateDynamicMaterialInstance` (`self.BrushPreview`) 0 null "None"))
  (set `self.BrushPreviewMID` _returnvalue)
  (bind _asbp_wheel_menu_01 (cast `/ShaderBits-GDC-Pack/PaintingVolumeTextures/Blueprints/HUD/RadialMenu/Blueprints/BP_WheelMenu_01` (`ChildActorComponent.ChildActor` (`self.ChildActor`))))
  (set `self.RadialMenu` _asbp_wheel_menu_01))

(event `Key|LeftMouseButton`
  (params (Key :type "Key Structure"))
  (bind _fluidsimbp (`self.FluidSimBP`))
  (:`Pressed`
    (`self.Line Trace Under Cursor`)
    (`|SpawnActorFromClass` "/Volumetrics/Tools/FluidSimulation/Blueprints/Pawn/FakeDecal.FakeDecal_C" (`KismetMathLibrary.Conv_VectorToTransform` (`self.Hit Position`)) "Undefined" "OverrideRootScale" null null))
  (:`Released`
    (set `self.Pressed` false)
    (`/Engine/EditorBlueprintResources/StandardMacros.IsValid` _fluidsimbp
      (:`Is Valid`
        (set `/Volumetrics/Tools/FluidSimulation/Blueprints/BP_FluidSimulation_01.Force Velocity` (0.0 0.0 0.0) _fluidsimbp)))))

(event `Key|RightMouseButton`
  (params (Key :type "Key Structure"))
  (bind _fluidsimbp (`self.FluidSimBP`))
  (:`Pressed`
    (set `self.Right` true)
    (set `/Volumetrics/Tools/FluidSimulation/Blueprints/BP_FluidSimulation_01.RightClick` true _fluidsimbp))
  (:`Released`
    (set `self.Right` false)
    (set `/Volumetrics/Tools/FluidSimulation/Blueprints/BP_FluidSimulation_01.RightClick` false _fluidsimbp)))

(event `self.ReceiveTick`
  (params (DeltaSeconds :type "Float (single-precision)"))
  (bind _fluidsimbp (`self.FluidSimBP`))
  (`self.Line Trace Under Cursor`)
  (`self.Update Brush Preview`)
  (if (`self.Pressed`)
    (set `self.Velocity` (* (`self.MouseVelocity`) (`self.Opacity`)))
    (if (== (`self.Hit Actor`) (`self.FlowMapBP`))
      (`/Engine/EditorBlueprintResources/StandardMacros.IsValid` (`self.FlowMapBP`)
        (:`Is Valid`
          (set `/ShaderBits-GDC-Pack/FlowMapPainter/BP_PaintFlowMap.Force Location` (`self.Hit Position`) (`self.FlowMapBP`))
          (set `/ShaderBits-GDC-Pack/FlowMapPainter/BP_PaintFlowMap.Force Velocity` (`self.Velocity`) (`self.FlowMapBP`))
          (set `/ShaderBits-GDC-Pack/FlowMapPainter/BP_PaintFlowMap.Brush Size` (`self.BrushSize`) (`self.FlowMapBP`))
          (`/ShaderBits-GDC-Pack/FlowMapPainter/BP_PaintFlowMap.Draw` (`self.FlowMapBP`))))
      (else
        (if (not (== (`self.Hit Actor`) _fluidsimbp))
          (`/Engine/EditorBlueprintResources/StandardMacros.IsValid` _fluidsimbp
            (:`Is Valid`
              _)))
        (set `/Volumetrics/Tools/FluidSimulation/Blueprints/BP_FluidSimulation_01.Obstacle Location` (`self.Hit Position`) (`self.FluidSimBP`))
        (set `/Volumetrics/Tools/FluidSimulation/Blueprints/BP_FluidSimulation_01.Force Velocity` (`self.MouseVelocity`) (`self.FluidSimBP`))
        (set `/Volumetrics/Tools/FluidSimulation/Blueprints/BP_FluidSimulation_01.Obstacle Radius` (* (`self.BrushSize`) 0.5) (`self.FluidSimBP`))))
    (elif (`self.Right`)
      (set `/Volumetrics/Tools/FluidSimulation/Blueprints/BP_FluidSimulation_01.Force Location` (`self.Hit Position`) (`self.FluidSimBP`)))))

(event `/ShaderBits-GDC-Pack/PaintingVolumeTextures/Blueprints/HUD/RadialMenu/Interface/RadialMenuBP_Interface.RadialMenu Action or Mode Change`
  (params (`New State` :type "/ShaderBits-GDC-Pack/PaintingVolumeTextures/Blueprints/HUD/RadialMenu/Enums/E_RadialMenu_StateChanges Enum" :default "NewEnumerator0") (Index :type Integer))
  (bind _returnvalue (`KismetStringLibrary.Conv_IntToString` Index))
  (switch `/ShaderBits-GDC-Pack/PaintingVolumeTextures/Blueprints/HUD/RadialMenu/Enums/E_RadialMenu_StateChanges` `New State`
    (:`NewEnumerator0`
      (`KismetSystemLibrary.PrintString` (`KismetStringLibrary.Concat_StrStr` "PAWN MODE SAYS: " _returnvalue)))
    (:`NewEnumerator1`
      (`KismetSystemLibrary.PrintString` (`KismetStringLibrary.Concat_StrStr` "PAWN ACTION #: " _returnvalue)))))

(event `Key|MouseScrollUp`
  (params (Key :type "Key Structure"))
  (bind _fluidsimbp (`self.FluidSimBP`))
  ;[1 1 1] Brush Settings
  (:`Pressed`
    (set `self.BrushSize` (* (`self.BrushSize`) 1.1))
    (`SceneComponent.SetWorldScale3D` (`self.BrushPreview`) (`KismetMathLibrary.Conv_DoubleToVector` (* (`self.BrushSize`) 250.0)))
    (`/Engine/EditorBlueprintResources/StandardMacros.IsValid` _fluidsimbp :!label _label
      (:`Is Valid`
        (set `/Volumetrics/Tools/FluidSimulation/Blueprints/BP_FluidSimulation_01.Obstacle Radius` (* (`self.BrushSize`) 0.5) _fluidsimbp)))))

(event `Key|Zero`
  (params (Key :type "Key Structure"))
  ;[1 1 1] Radial Menu Keyboard Debug
  (:`Pressed`
    (`/ShaderBits-GDC-Pack/PaintingVolumeTextures/Blueprints/HUD/RadialMenu/Blueprints/BP_WheelMenu_01.Manual Selection` (`self.RadialMenu`) 0)))

(event `Key|MouseScrollDown`
  (params (Key :type "Key Structure"))
  ;[1 1 1] Brush Settings
  (:`Pressed`
    (set `self.BrushSize` (* (`self.BrushSize`) 0.9))
    (`SceneComponent.SetWorldScale3D` (`self.BrushPreview`) (`KismetMathLibrary.Conv_DoubleToVector` (* (`self.BrushSize`) 250.0)))
    (goto _label)))

(event `Key|One`
  (params (Key :type "Key Structure"))
  ;[1 1 1] Radial Menu Keyboard Debug
  (:`Pressed`
    (`/ShaderBits-GDC-Pack/PaintingVolumeTextures/Blueprints/HUD/RadialMenu/Blueprints/BP_WheelMenu_01.Manual Selection` (`self.RadialMenu`) 1)))

(event `Key|Two`
  (params (Key :type "Key Structure"))
  ;[1 1 1] Radial Menu Keyboard Debug
  (:`Pressed`
    (`/ShaderBits-GDC-Pack/PaintingVolumeTextures/Blueprints/HUD/RadialMenu/Blueprints/BP_WheelMenu_01.Manual Selection` (`self.RadialMenu`) 2)))

(event `Key|A`
  (params (Key :type "Key Structure"))
  ;[1 1 1] Brush Settings
  (:`Pressed`
    (set `self.Opacity` (+ (`self.Opacity`) 0.1))
    (`MaterialInstanceDynamic.SetScalarParameterValue` (`self.BrushPreviewMID`) "Opacity" (`self.Opacity`) :!label _label_2)))

(event `Key|Three`
  (params (Key :type "Key Structure"))
  ;[1 1 1] Radial Menu Keyboard Debug
  (:`Pressed`
    (`/ShaderBits-GDC-Pack/PaintingVolumeTextures/Blueprints/HUD/RadialMenu/Blueprints/BP_WheelMenu_01.Manual Selection` (`self.RadialMenu`) 3)))

(event `Key|Z`
  (params (Key :type "Key Structure"))
  ;[1 1 1] Brush Settings
  (:`Pressed`
    (set `self.Opacity` (+ (`self.Opacity`) -0.1))
    (goto _label_2)))

(fn `Line Trace Under Cursor`
  (bind (_hitresult _returnvalue) (`PlayerController.GetHitResultUnderCursorByChannel` (`GameplayStatics.GetPlayerController` 0) "TraceTypeQuery1" true))
  (bind (_bblockinghit _binitialoverlap _time _distance _location _impactpoint _normal _impactnormal _physmat _hitactor) (`GameplayStatics.BreakHitResult` _hitresult))
  (if _returnvalue
    (set `self.MouseVelocity` (- _location (`self.Hit Position`)))
    (set `self.Hit Position` _location)
    (set `self.Hit Actor` _hitactor)))

(fn `Update Brush Preview`
  (`SceneComponent.K2_SetWorldLocation` (`self.BrushPreview`) (`self.Hit Position`) false false))

(fn `UserConstructionScript`)